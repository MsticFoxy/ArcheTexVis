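; VTT_targetObject is a child Blueprint that defines a vector pointing from a tracked actor toward a TargetObject.
; GetDirection returns the unnormalized offset between the two actors' locations.
; GetLength returns either a fixed Length or that offset's distance, depending on UseFixedLength.
; Both fall back to the parent implementation without a valid target, while GetPosition always defers to the parent.
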(fn `GetDirection`
  (returns (direction :type "Vector Structure"))
  (bind _targetobject (`self.TargetObject`))
  (`/Engine/EditorBlueprintResources/StandardMacros.IsValid` _targetobject
    (:`Is Valid`
      (return (- (`Actor.K2_GetActorLocation` _targetobject) (`Actor.K2_GetActorLocation` (`self.GetTracked`)))))
    (:`Is Not Valid`
      (return (`parent.GetDirection`)))))

(fn `GetLength`
  (returns (length :type "Float (double-precision)"))
  (bind _targetobject (`self.TargetObject`))
  (`/Engine/EditorBlueprintResources/StandardMacros.IsValid` _targetobject
    (:`Is Valid`
      (return (select `bool` (`self.useFixedLength`) :`false` (`KismetMathLibrary.VSize` (- (`Actor.K2_GetActorLocation` _targetobject) (`Actor.K2_GetActorLocation` (`self.GetTracked`)))) :`true` (`self.length`))))
    (:`Is Not Valid`
      (return (`parent.GetLength`)))))

(fn `GetPosition`
  (returns (position :type "Vector Structure"))
  (return (`parent.GetPosition`)))