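; OrbitControl is a mouse-driven orbit camera actor that also toggles the Project Explorer in the MaterialScannerControlUI widget.
; Mouse axes feed Orbit, which yaws the actor in world space and pitches CamDirection within a clamped downward range.
; BeginPlay shows the cursor and sets Game and UI input.
; MovementActivate sets an InMovement flag, but Orbit does not check it, so mouse motion always rotates the view.
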(event `self.ReceiveBeginPlay`
  (bind _returnvalue (`GameplayStatics.GetPlayerController` 0))
  (set `PlayerController.bShowMouseCursor` true _returnvalue)
  (`WidgetBlueprintLibrary.SetInputMode_GameAndUIEx` _returnvalue null "DoNotLock" false))

(event `InputAction|MovementActivate`
  (params (Key :type "Key Structure"))
  (:`Pressed`
    (set `self.inMovement` true))
  (:`Released`
    (set `self.inMovement` false)))

(event `InputAxis|MouseX`
  (params (AxisValue :type "Float (single-precision)"))
  (`self.Orbit` (`KismetMathLibrary.MakeVector2D` AxisValue)))

(event `InputAxis|MouseY`
  (params (AxisValue :type "Float (single-precision)"))
  (`self.Orbit` (`KismetMathLibrary.MakeVector2D` 0.0 AxisValue)))

(event `InputAction|ToggleProjectExplorer`
  (params (Key :type "Key Structure"))
  (:`Pressed`
    (bind _returnvalue (`VictoryBPFunctionLibrary.GetFirstWidgetOfClass` "/Game/Blueprints/UI/MaterialScannerControlUI.MaterialScannerControlUI_C"))
    (`/Engine/EditorBlueprintResources/StandardMacros.IsValid` _returnvalue
      (:`Is Valid`
        (`/Game/Blueprints/UI/MaterialScannerControlUI.ToggleProjectExplorer` _returnvalue)))))

(fn `Orbit`
  (params (orbitInput :type "Vector2D Structure"))
  (bind _camdirection (`self.CamDirection`))
  (bind (_relativerotation_roll _relativerotation_pitch) (`KismetMathLibrary.BreakRotator` (`SceneComponent.RelativeRotation` _camdirection)))
  (`self.K2_AddActorWorldRotation` (`KismetMathLibrary.MakeRotator` 0.0 0.0 (* orbitInput_X 5.0)))
  (`SceneComponent.K2_SetRelativeRotation` _camdirection (`KismetMathLibrary.MakeRotator` 0.0 (`KismetMathLibrary.FClamp` (+ _relativerotation_pitch (* orbitInput_Y 5.0)) -80.0 -15.0)) false false))

(fn `UserConstructionScript`)