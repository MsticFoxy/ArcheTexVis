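; Actor that draws a colored 3D arrow visualizing a vector, updated during play and in the editor.
; Construction gathers VectorTrackingType components from itself or an override actor; these supply position, direction and length, the last overriding component winning.
; Each update moves the actor, rotates the arrow and fits stem and tip to length, optionally setting itself as the components' tracked actor.
; Color comes from a dynamic unlit material.
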(event `self.ReceiveTick`
  (params (DeltaSeconds :type "Float (single-precision)"))
  (`self.UpdateArrow`))

(event `self.BlueprintEditorTick`
  (params (DeltaTime :type "Float (single-precision)"))
  (`self.UpdateArrow`))

(fn `Get Direction`
  (returns (direction :type "Vector Structure"))
  (locals (dir :type "Vector Structure"))
  (set `local.dir` (1.0 0.0 0.0))
  (for _array_element (`self.trackingType`)
    (if (`/Game/Blueprints/VectorTrackingType.overrideDirection` _array_element)
      (`self.OverrideTrackingActor` self _array_element)
      (set `local.dir` (`/Game/Blueprints/VectorTrackingType.GetDirection` _array_element))))
  (return (`local.dir`)))

(fn `GetLength`
  (returns (length :type "Float (double-precision)"))
  (locals (len :type "Float (double-precision)"))
  (set `local.len` 100.0)
  (for _array_element (`self.trackingType`)
    (if (`/Game/Blueprints/VectorTrackingType.overrideLength` _array_element)
      (`self.OverrideTrackingActor` self _array_element)
      (set `local.len` (`/Game/Blueprints/VectorTrackingType.GetLength` _array_element))))
  (return (`local.len`)))

(fn `GetPosition`
  (returns (position :type "Vector Structure"))
  (locals (pos :type "Vector Structure"))
  (set `local.pos` (`self.K2_GetActorLocation`))
  (for _array_element (`self.trackingType`)
    (if (`/Game/Blueprints/VectorTrackingType.overridePosition` _array_element)
      (`self.OverrideTrackingActor` self _array_element)
      (set `local.pos` (`/Game/Blueprints/VectorTrackingType.GetPosition` _array_element))))
  (return (`local.pos`)))

(fn `OverrideTrackingActor`
  (params (Target :type "/Game/Blueprints/VectorTrackingType Object Reference"))
  (if (`self.allowOverrideTrackingActor`)
    (set `/Game/Blueprints/VectorTrackingType.overrideTrackedActor` self Target)))

(fn `SetColor`
  (params (color :type "LinearColor Structure"))
  (set `self.color` color)
  (`/Engine/EditorBlueprintResources/StandardMacros.IsValid` (`self.dynamicMat`)
    (:`Is Valid`
      _)
    (:`Is Not Valid`
      (bind _returnvalue (`KismetMaterialLibrary.CreateDynamicMaterialInstance` "/Game/Models/UnlitBasicColor.UnlitBasicColor"))
      (bind _output_get (set `self.dynamicMat` _returnvalue))
      (`PrimitiveComponent.SetMaterial` (`self.ArrowStem`) 0 _output_get)
      (`PrimitiveComponent.SetMaterial` (`self.ArrowTip`) 0 _output_get)))
  (`MaterialInstanceDynamic.SetVectorParameterValue` (`self.dynamicMat`) "Color" color))

(fn `UpdateArrow`
  (bind _length (`self.GetLength`))
  (`self.K2_SetActorLocation` (`self.GetPosition`))
  (`SceneComponent.K2_SetWorldRotation` (`self.ArrowRoot`) (`KismetMathLibrary.FindLookAtRotation` (0.0 0.0 0.0) (`self.Get Direction`)) false false)
  (`SceneComponent.SetRelativeScale3D` (`self.ArrowStem`) (`KismetMathLibrary.MakeVector` 1.0 1.0 (* (- _length 10.0) 0.01)))
  (`SceneComponent.K2_SetRelativeLocation` (`self.ArrowTip`) (`KismetMathLibrary.MakeVector` (- _length 20.0)) false false))

(fn `UserConstructionScript`
  (`/Engine/EditorBlueprintResources/StandardMacros.IsValid` (`self.overrideTrackingTypeActor`)
    (:`Is Valid`
      (set `self.trackingType` (`self.K2_GetComponentsByClass` (`self.overrideTrackingTypeActor`) "/Game/Blueprints/VectorTrackingType.VectorTrackingType_C")))
    (:`Is Not Valid`
      (set `self.trackingType` (`self.K2_GetComponentsByClass` "/Game/Blueprints/VectorTrackingType.VectorTrackingType_C"))))
  (`self.UpdateArrow`)
  (`self.SetColor` (`self.color`)))