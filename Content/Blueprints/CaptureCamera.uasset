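; Capture camera actor that renders its scene capture component to a render target and exports it as a named PNG under the project's Captures/SingleCaptures folder.
; CaptureImage validates the target texture, captures, exports, then broadcasts OnImageCaptured.
; SetUpExposure enables every-frame capture for a short countdown on editor tick, apparently letting exposure settle outside play.
; The construction script raises an arrow component by Height.
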(event `self.ReceiveBeginPlay`)

(event `Caprture`
  (`self.CaptureImage` (`KismetStringLibrary.Concat_StrStr` (`KismetSystemLibrary.GetProjectDirectory`) "Captures/SingleCaptures/") (`KismetStringLibrary.Concat_StrStr` (`self.singleCaptureName`) ".png")))

(event `SetUpExposure`
  (set `SceneCaptureComponent.bCaptureEveryFrame` true (`self.SceneCaptureComponent2D`))
  (set `self.exposureTimer` 5.0))

(event `self.BlueprintEditorTick`
  (params (DeltaTime :type "Float (single-precision)"))
  (bind _exposuretimer (`self.exposureTimer`))
  (if (> _exposuretimer 0.0)
    (bind _output_get (set `self.exposureTimer` (- _exposuretimer DeltaTime)))
    (if (<= _output_get 0.0)
      (set `SceneCaptureComponent.bCaptureEveryFrame` false (`self.SceneCaptureComponent2D`)))))

(fn `CaptureImage`
  (params (path :type String) (filename :type String))
  (bind _scenecapturecomponent2d (`self.SceneCaptureComponent2D`))
  (bind _texturetarget (`SceneCaptureComponent2D.TextureTarget` _scenecapturecomponent2d))
  (`/Engine/EditorBlueprintResources/StandardMacros.IsValid` _texturetarget
    (:`Is Valid`
      (`SceneCaptureComponent2D.CaptureScene` _scenecapturecomponent2d)
      (`KismetRenderingLibrary.ExportRenderTarget` _texturetarget path filename)
      (`self.OnImageCaptured`))
    (:`Is Not Valid`
      (`KismetSystemLibrary.PrintString` "No Target Texture"))))

(fn `UserConstructionScript`
  (`SceneComponent.K2_AddLocalOffset` (`self.Arrow`) (`KismetMathLibrary.MakeVector` 0.0 0.0 (`self.height`)) false false))