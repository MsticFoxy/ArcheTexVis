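; Actor that captures an image per light direction by lighting each VV_LightVector of an AnimationRing in turn, with the HeadLight hidden.
; A countdown driven by game and editor ticks steps the lights, triggering CaptureCamera midway through each interval.
; Filenames encode each light's azimuth and elevation, saved under Captures/Test.
; Completion restores the HeadLight and fires a callback; a separate CalculateTextures event shells out to an external program.
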(event `self.ReceiveBeginPlay`)

(event `self.ReceiveTick`
  (params (DeltaSeconds :type "Float (single-precision)"))
  (`self.AnimationTick` DeltaSeconds))

(event `self.BlueprintEditorTick`
  (params (DeltaTime :type "Float (single-precision)"))
  (`self.AnimationTick` DeltaTime))

(event `AnimationTick`
  (params (delta :type "Float (double-precision)"))
  (bind _capturecamera (`self.CaptureCamera`))
  (bind _remtime (`self.remTime`))
  (bind (_filepath _filename) (`self.GetFilePathByID` (`self.currentID`)))
  (if (> _remtime 0.0)
    (bind _output_get (set `self.remTime` (- _remtime delta)))
    (if (< _output_get (/ (`self.lightActiveTime`) 2.0))
      (`/Engine/EditorBlueprintResources/StandardMacros.IsValid` _capturecamera
        (:`Is Valid`
          (if (not (`self.captured`))
            (set `self.captured` true)
            (`/Game/Blueprints/CaptureCamera.CaptureImage` _capturecamera _filepath _filename)))))
    (elif (`self.activateInvoke`)
      (set `self.activateInvoke` false)
      (`self.InvokeStep`))))

(event `RunAnimation`
  (bind _animationring (`self.AnimationRing`))
  (set `self.animRunning` true)
  (`/Engine/EditorBlueprintResources/StandardMacros.IsValid` _animationring
    (:`Is Valid`
      (for _array_element (`/Game/Blueprints/VectorRing.vectorActors` _animationring)
        (bind _asvv_light_vector (cast `/Game/Blueprints/VV_LightVector` _array_element))
        (`/Game/Blueprints/VV_LightVector.SetEmitLight` _asvv_light_vector false))
      (`self.SetHeadLightVisibility` false)
      (`self.RunIndex` 0))))

(event `RunIndex`
  (params (index :type Integer))
  (bind _animationring (`self.AnimationRing`))
  (bind _vectoractors (`/Game/Blueprints/VectorRing.vectorActors` _animationring))
  (`/Engine/EditorBlueprintResources/StandardMacros.IsValid` _animationring
    (:`Is Valid`
      (if (> (`KismetArrayLibrary.Array_Length` _vectoractors) index)
        (bind _asvv_light_vector (cast `/Game/Blueprints/VV_LightVector` (`|GetArrayItem` _vectoractors index)))
        (`/Game/Blueprints/VV_LightVector.SetEmitLight` _asvv_light_vector true)
        (set `self.currentID` index)
        (set `self.CurrentLight` _asvv_light_vector)
        (set `self.remTime` (`self.lightActiveTime`))
        (set `self.activateInvoke` true)
        (set `self.captured` false)
        (else
          (`self.EndAnimation`))))))

(event `InvokeStep`
  (bind _returnvalue (+ (`self.currentID`) 1))
  (`/Game/Blueprints/VV_LightVector.SetEmitLight` (`self.CurrentLight`) false)
  (if (>= _returnvalue (`KismetArrayLibrary.Array_Length` (`/Game/Blueprints/VectorRing.vectorActors` (`self.AnimationRing`))))
    (`self.EndAnimation`)
    (else
      (`self.RunIndex` _returnvalue))))

(event `EndAnimation`
  (bind _animationring (`self.AnimationRing`))
  (`/Engine/EditorBlueprintResources/StandardMacros.IsValid` _animationring
    (:`Is Valid`
      (for _array_element (`/Game/Blueprints/VectorRing.vectorActors` _animationring)
        (bind _asvv_light_vector (cast `/Game/Blueprints/VV_LightVector` _array_element))
        (`/Game/Blueprints/VV_LightVector.SetEmitLight` _asvv_light_vector false))
      (`self.OnAnimationComplete`)
      (`self.SetHeadLightVisibility` true))))

(event `CalculateTextures`
  (bind _returnvalue (`KismetStringLibrary.Concat_StrStr` (`self.ProgramLocation`) " " (`self.CalculationDirectory`) " " (`self.OutputFileDirectory`) (`self.OutputFileName`) ".png" " " "15"))
  (`KismetSystemLibrary.PrintString` _returnvalue)
  (`ImageManagementLibrary.ShellCommand` _returnvalue))

(event `ActivateSingleLight`
  (bind _animationring (`self.AnimationRing`))
  (`/Engine/EditorBlueprintResources/StandardMacros.IsValid` _animationring
    (:`Is Valid`
      (for (_array_element _array_index) (`/Game/Blueprints/VectorRing.vectorActors` _animationring)
        (bind _asvv_light_vector (cast `/Game/Blueprints/VV_LightVector` _array_element))
        (`/Game/Blueprints/VV_LightVector.SetEmitLight` _asvv_light_vector (== _array_index 0))))))

(fn `GetFilePathByID`
  (params (id :type Integer))
  (returns (FilePath :type String) (FileName :type String))
  (bind _returnvalue (`KismetStringLibrary.Concat_StrStr` (`KismetSystemLibrary.GetProjectDirectory`) "Captures/Test/"))
  (bind _asvv_light_vector (cast `/Game/Blueprints/VV_LightVector` (`|GetArrayItem` (`/Game/Blueprints/VectorRing.vectorActors` (`self.AnimationRing`)) id))
    (:`then`
      (return _returnvalue (`self.WriteFileName` "test" _asvv_light_vector)))
    (:`CastFailed`
      (return _returnvalue "test"))))

(fn `SetHeadLightVisibility`
  (params (visible :type Boolean))
  (bind _headlight (`self.HeadLight`))
  (`/Engine/EditorBlueprintResources/StandardMacros.IsValid` _headlight
    (:`Is Valid`
      (`SceneComponent.SetVisibility` (`Light.LightComponent` _headlight) visible false))))

(fn `UserConstructionScript`)

(fn `WriteFileName`
  (params (baseName :type String) (light :type "/Game/Blueprints/VV_LightVector Object Reference"))
  (returns (name :type String))
  (bind _direction (`/Game/Blueprints/VisualizationVector.Get Direction` light))
  (bind (_returnvalue_x _returnvalue_y) (`KismetMathLibrary.BreakVector` (`KismetMathLibrary.RotateAngleAxis` _direction -90.0 (0.0 0.0 1.0))))
  (bind (_returnvalue_roll _returnvalue_pitch _returnvalue_yaw) (`KismetMathLibrary.BreakRotator` (`KismetMathLibrary.FindLookAtRotation` (0.0 0.0 0.0) (`KismetMathLibrary.MakeVector` _returnvalue_x _returnvalue_y))))
  (return (`KismetStringLibrary.Concat_StrStr` baseName "_" (`KismetTextLibrary.Conv_TextToString` (`KismetTextLibrary.Conv_DoubleToText` (`KismetMathLibrary.Abs` (+ _returnvalue_yaw -180.0)) "HalfToEven" false true 3 3 0 0)) "_" (`KismetTextLibrary.Conv_TextToString` (`KismetTextLibrary.Conv_DoubleToText` (`KismetMathLibrary.DegAcos` (/ (`KismetMathLibrary.Dot_VectorVector` (`KismetMathLibrary.Normal` _direction) (`KismetMathLibrary.Normal` (`KismetMathLibrary.MakeVector` (.x _direction) (.y _direction)))) 1.0)) "HalfToEven" false true 3 3 0 0)) ".png")))