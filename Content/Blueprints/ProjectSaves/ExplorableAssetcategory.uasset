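; ExplorableAssetcategory is a project-save category that holds a collection of assets in a map keyed by asset name.
; AddAsset registers a new asset and binds to its rename event, or signals OnAssetAlreadyExists when that name is taken.
; Renaming re-keys the map entry and notifies the owning project of the change.
; GetAssets and GetAssetByName expose the stored assets for lookup.
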(event `AddAsset`
  (params (asset :type "/Game/Blueprints/ProjectSaves/ExplorableAsset Object Reference"))
  (bind _name (`/Game/Blueprints/ProjectSaves/ExplorableAsset.GetAssetName` asset))
  (bind _assets (`self.assets`))
  (bind (_value _returnvalue) (`BlueprintMapLibrary.Map_Find` _assets _name))
  (if _returnvalue
    (`self.OnAssetAlreadyExists` asset _value)
    (else
      (`BlueprintMapLibrary.Map_Add` _assets _name asset)
      (add `/Game/Blueprints/ProjectSaves/ExplorableAsset.OnRename` asset (delegate `RenameAsset`)))))

(event `RenameAsset`
  (params (asset :type "/Game/Blueprints/ProjectSaves/ExplorableAsset Object Reference") (oldName :type String) (newName :type String) (NewParam :type Boolean))
  (bind _assets (`self.assets`))
  (`BlueprintMapLibrary.Map_Remove` _assets oldName)
  (`BlueprintMapLibrary.Map_Add` _assets newName asset)
  (`/Game/Blueprints/ProjectSaves/Project.NotifyChange` (`/Game/Blueprints/ProjectSaves/ExplorableAsset.GetProject` asset)))

(fn `GetAssetByName`
  (params (name :type String))
  (returns (asset :type "/Game/Blueprints/ProjectSaves/ExplorableAsset Object Reference"))
  (bind (_value _returnvalue) (`BlueprintMapLibrary.Map_Find` (`self.assets`) name))
  (if _returnvalue
    (return _value)
    (else
      (return null))))

(fn `GetAssets`
  (returns (assets :type "Array of /Game/Blueprints/ProjectSaves/ExplorableAsset Object Reference"))
  (bind _values (`BlueprintMapLibrary.Map_Values` (`self.assets`)))
  (return _values))