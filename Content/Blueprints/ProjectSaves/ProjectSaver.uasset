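; ProjectSaver is an actor that creates, saves and loads a ProjectSave holding a Project of assets, firing OnLoaded with the project.
; BeginPlay always builds a fresh project, filled with numbered test assets for each entry in Classes, named from the trimmed class name.
; OnLoaded follows a short Delay in the class loop.
; LoadSave reads the named slot synchronously, while SaveGame writes it asynchronously.
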(event `self.ReceiveBeginPlay`
  (`self.CreateNewProject`))

(event `LoadSave`
  (bind _returnvalue (`GameplayStatics.LoadGameFromSlot` (`self.slotName`)))
  (bind _asproject_save (cast `/Game/Blueprints/ProjectSaves/ProjectSave` _returnvalue))
  (set `self.save` _asproject_save)
  (`self.OnLoaded` (`/Game/Blueprints/ProjectSaves/ProjectSave.project` (`self.save`))))

(event `SaveGame`
  (`AsyncActionHandleSaveGame.AsyncSaveGameToSlot` (`self.save`) (`self.slotName`)))

(event `CreateNewProject`
  (bind _returnvalue (`GameplayStatics.CreateSaveGameObject` "/Game/Blueprints/ProjectSaves/ProjectSave.ProjectSave_C"))
  (bind _output_get (set `self.save` _returnvalue))
  (bind _returnvalue_2 (`|GenericCreateObject` "/Game/Blueprints/ProjectSaves/Project.Project_C" _output_get))
  (bind _output_get_2 (set `/Game/Blueprints/ProjectSaves/ProjectSave.project` _returnvalue_2 _output_get))
  (for _array_element (`self.classes`)
    (for _index (range 11)
      (bind _returnvalue_3 (`|GenericCreateObject` _array_element _output_get_2))
      (bind _returnvalue_4 (`KismetSystemLibrary.GetClassDisplayName` _array_element))
      (`/Game/Blueprints/ProjectSaves/ExplorableAsset.RenameAsset` _returnvalue_3 (`KismetStringLibrary.Concat_StrStr` (`KismetStringLibrary.Concat_StrStr` "Test." (`KismetStringLibrary.GetSubstring` _returnvalue_4 0 (- (`KismetStringLibrary.Len` _returnvalue_4) 2))) "_" (`KismetStringLibrary.Conv_IntToString` _index)) true)
      (`/Game/Blueprints/ProjectSaves/Project.AddAsset` _output_get_2 _returnvalue_3))
    (`KismetSystemLibrary.Delay` 0.2)
    (`self.OnLoaded` (`/Game/Blueprints/ProjectSaves/ProjectSave.project` (`self.save`)))))

(fn `UserConstructionScript`)