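; Project object in the save system that holds assets in a map of ExplorableAssetCategory objects keyed by asset class.
; AddAsset links the asset to the project, binds its rename event, fires OnChange, then files it in its category, creating one if missing.
; Successful renames also fire OnChange through NotifyChange.
; GetAssetByName delegates name lookups to the category matching the given class.
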(event `BindAssetEvents`
  (params (asset :type "/Game/Blueprints/ProjectSaves/ExplorableAsset Object Reference"))
  (add `/Game/Blueprints/ProjectSaves/ExplorableAsset.OnRename` asset (delegate `OnRename`)))

(event `OnRename`
  (params (asset :type "/Game/Blueprints/ProjectSaves/ExplorableAsset Object Reference") (oldName :type String) (newName :type String) (success :type Boolean))
  (if success
    (`self.NotifyChange`)))

(fn `AddAsset`
  (params (asset :type "/Game/Blueprints/ProjectSaves/ExplorableAsset Object Reference"))
  (bind _returnvalue (`GameplayStatics.GetObjectClass` asset))
  (bind (_value _returnvalue_2) (`BlueprintMapLibrary.Map_Find` (`self.assets`) _returnvalue))
  (`/Game/Blueprints/ProjectSaves/ExplorableAsset.SetProject` asset self)
  (`self.BindAssetEvents` asset)
  (`self.OnChange`)
  (if _returnvalue_2
    (`/Game/Blueprints/ProjectSaves/ExplorableAssetcategory.AddAsset` _value asset)
    (else
      (bind _returnvalue_3 (`|GenericCreateObject` "/Game/Blueprints/ProjectSaves/ExplorableAssetcategory.ExplorableAssetCategory_C" self))
      (`BlueprintMapLibrary.Map_Add` (`self.assets`) _returnvalue _returnvalue_3)
      (`/Game/Blueprints/ProjectSaves/ExplorableAssetcategory.AddAsset` _returnvalue_3 asset))))

(fn `GetAssetByName`
  (params (categoryClass :type "/Game/Blueprints/ProjectSaves/ExplorableAsset Class Reference") (name :type String))
  (returns (asset :type "/Game/Blueprints/ProjectSaves/ExplorableAsset Object Reference"))
  (bind (_value _returnvalue) (`BlueprintMapLibrary.Map_Find` (`self.assets`) categoryClass))
  (if _returnvalue
    (bind _asset (`/Game/Blueprints/ProjectSaves/ExplorableAssetcategory.GetAssetByName` _value name))
    (return _asset)
    (else
      (return null))))

(fn `NotifyChange`
  (`self.OnChange`))