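; ExplorableAsset is a named asset belonging to a Project, with an empty GetInspectorWidget function that returns nothing here.
; Renaming fails if the Project already holds an asset of the same class with that name; without a valid Project it always succeeds.
; Unless suppressed, both outcomes fire OnRename with old and new names.
; Names are dot-delimited paths, with the last segment used as display name.
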(fn `GetAssetDisplayName`
  (returns (name :type String))
  (bind _returnvalue (`KismetStringLibrary.ParseIntoArray` (`self.GetAssetName`) "."))
  (return (`|GetArrayItem` _returnvalue (- (`KismetArrayLibrary.Array_Length` _returnvalue) 1))))

(fn `GetAssetName`
  (returns (name :type String))
  (return (`self.AssetName`)))

(fn `GetInspectorWidget`
  (returns (widget :type "UserWidget Object Reference"))
  (return null))

(fn `GetProject`
  (returns (project :type "/Game/Blueprints/ProjectSaves/Project Object Reference"))
  (return (`self.project`)))

(fn `RenameAsset`
  (params (newName :type String) (skipRenameNotification :type Boolean))
  (locals (oldName :type String))
  (bind _project (`self.project`))
  (bind _output_get (set `local.oldName` (`self.GetAssetName`)))
  (`/Engine/EditorBlueprintResources/StandardMacros.IsValid` _project
    (:`Is Valid`
      (bind _asset (`/Game/Blueprints/ProjectSaves/Project.GetAssetByName` _project (`GameplayStatics.GetObjectClass` self) newName))
      (`/Engine/EditorBlueprintResources/StandardMacros.IsValid` _asset
        (:`Is Valid`
          (if (not skipRenameNotification)
            (`self.OnRename` self _output_get newName)))
        (:`Is Not Valid`
          (bind _output_get_2 (set `self.AssetName` newName :!label _label))
          (if (not skipRenameNotification)
            (`self.OnRename` self _output_get _output_get_2 true)))))
    (:`Is Not Valid`
      (goto _label))))

(fn `SetProject`
  (params (project :type "/Game/Blueprints/ProjectSaves/Project Object Reference"))
  (set `self.project` project))