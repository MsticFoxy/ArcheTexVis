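; VectorRing is an actor that spawns and manages a ring of colored vector actors around itself.
; GenerateVectors, when the count is positive, destroys the previous set, then spawns, colors and attaches new actors of the configured class.
; Each is placed by rotating a radius vector through evenly spaced yaw angles plus an offset, while its rotation snaps to the ring's.
; Empty destroys all spawned actors and clears the list.
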(event `GenerateVectors`
  (bind _vectorcount (`self.vectorCount`))
  (if (> (`self.vectorCount`) 0)
    (for _array_element (`self.vectorActors`)
      (`self.K2_DestroyActor` _array_element))
    (`KismetArrayLibrary.Array_Clear` (`self.vectorActors`))
    (for _index (range 1 (+ _vectorcount 1))
      (bind _returnvalue (`|SpawnActorFromClass` (`self.vectorClass`) (`KismetMathLibrary.MakeTransform` (0.0 0.0 0.0)) "Undefined" "OverrideRootScale" null self null))
      (`/Game/Blueprints/VisualizationVector.SetColor` _returnvalue (`self.vectorColor`))
      (`KismetArrayLibrary.Array_AddUnique` (`self.vectorActors`) _returnvalue)
      (`self.K2_AttachToActor` _returnvalue self "None" "SnapToTarget" "SnapToTarget" "KeepRelative" true)
      (`self.K2_SetActorRelativeLocation` _returnvalue (+ (`KismetMathLibrary.GreaterGreater_VectorRotator` (`KismetMathLibrary.MakeVector` (`self.radius`)) (`KismetMathLibrary.MakeRotator` 0.0 0.0 (* (/ (`KismetMathLibrary.Conv_IntToDouble` _index) (`KismetMathLibrary.Conv_IntToDouble` _vectorcount)) 360.0))) (`self.offset`)) false false))))

(event `Empty`
  (for _array_element (`self.vectorActors`)
    (`self.K2_DestroyActor` _array_element))
  (`KismetArrayLibrary.Array_Clear` (`self.vectorActors`)))

(fn `UserConstructionScript`)