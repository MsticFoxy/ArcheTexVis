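; VectorTrackingType supplies a position, direction and length that describe a vector tracked from an actor.
; GetTracked returns OverrideTrackedActor when valid, otherwise the owner.
; GetPosition and GetDirection read that actor's location and forward vector, while GetLength returns a fixed constant.
; BeginPlay and Tick are unused, so values are computed only when the getters are called.
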(fn `GetDirection`
  (returns (direction :type "Vector Structure"))
  (return (`Actor.GetActorForwardVector` (`self.GetTracked`))))

(fn `GetLength`
  (returns (length :type "Float (double-precision)"))
  (return 100.0))

(fn `GetPosition`
  (returns (position :type "Vector Structure"))
  (return (`Actor.K2_GetActorLocation` (`self.GetTracked`))))

(fn `GetTracked`
  (returns (tracked :type "Actor Object Reference"))
  (bind _overridetrackedactor (`self.overrideTrackedActor`))
  (`/Engine/EditorBlueprintResources/StandardMacros.IsValid` _overridetrackedactor
    (:`Is Valid`
      (return _overridetrackedactor))
    (:`Is Not Valid`
      (return (`self.GetOwner`)))))