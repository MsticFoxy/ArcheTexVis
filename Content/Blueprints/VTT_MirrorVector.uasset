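; VTT_MirrorVector is a vector Blueprint that mirrors the direction, length and position of another vector, TargetVector.
; Its three getters return TargetVector's direction, length and actor location while that reference is valid.
; Without a valid target, they fall back to BasicDirection, BasicLength and the location of the actor returned by GetTracked.
; The event graph holds no active logic.
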(fn `GetDirection`
  (returns (direction :type "Vector Structure"))
  (bind _targetvector (`self.TargetVector`))
  (`/Engine/EditorBlueprintResources/StandardMacros.IsValid` _targetvector
    (:`Is Valid`
      (return (`/Game/Blueprints/VisualizationVector.Get Direction` _targetvector)))
    (:`Is Not Valid`
      (return (`self.basicDirection`)))))

(fn `GetLength`
  (returns (length :type "Float (double-precision)"))
  (bind _targetvector (`self.TargetVector`))
  (`/Engine/EditorBlueprintResources/StandardMacros.IsValid` _targetvector
    (:`Is Valid`
      (return (`/Game/Blueprints/VisualizationVector.GetLength` _targetvector)))
    (:`Is Not Valid`
      (return (`self.basicLength`)))))

(fn `GetPosition`
  (returns (position :type "Vector Structure"))
  (bind _targetvector (`self.TargetVector`))
  (`/Engine/EditorBlueprintResources/StandardMacros.IsValid` _targetvector
    (:`Is Valid`
      (return (`Actor.K2_GetActorLocation` _targetvector)))
    (:`Is Not Valid`
      (return (`Actor.K2_GetActorLocation` (`self.GetTracked`))))))